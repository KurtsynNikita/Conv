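; BP_SplineConveyor is an actor that builds a conveyor layout from child actors placed along a spline.
; Its construction script divides the spline length by StepLength and adds one Child Actor component per whole step.
; Each component takes its local location and rotation from the spline at that distance, with unit scale.
; The event graph holds only disabled placeholder events, so the graphs add no runtime movement.
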(event EventBeginPlay)

(event Collision|EventActorBeginOverlap
  (params (OtherActor :type Actor%20Object%20Reference)))

(fn ConstructionScript
  (bind _spline (Variables|Default|GetSpline))
  (for _index (range 0 (- (Math|Float|Truncate (/ (Spline|GetSplineLength (Variables|Default|GetSpline)) (Variables|Default|GetStepLength))) 1))
    (Variables|Default|SetIndex _index)
    (AddComponent|AddChildActorComponent false (Math|Transform|MakeTransform (Spline|GetLocationatDistanceAlongSpline _spline (* (Variables|Default|GetIndex) (Variables|Default|GetStepLength)) "Local") (Spline|GetRotationatDistanceAlongSpline _spline (* (Variables|Default|GetIndex) (Variables|Default|GetStepLength)) "Local") "1,1.000000,1"))))