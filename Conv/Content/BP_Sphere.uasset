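; BP_Sphere is a sphere item actor that exposes its type, speed, flash color and position along a path.
; A NewDistance event stores the current path distance, and getter functions return that distance, the "Sphere" type name, its movement speed and its flash color.
; It has no movement logic of its own; BeginPlay, overlap and Tick are unused.
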(event EventBeginPlay)

(event Collision|EventActorBeginOverlap
  (params (OtherActor :type Actor%20Object%20Reference)))

(event EventTick
  (params (DeltaSeconds :type Float%20%28single-precision%29)))

(event EventNewDistance
  (params (New%20Distance :type Float%20%28single-precision%29))
  (Variables|Default|SetCurrentPathDistance New%20Distance))

(fn ConstructionScript)

(fn GetCurrentDistance
  (return (Variables|Default|GetCurrentPathDistance)))

(fn GetItemType
  (return "Sphere"))

(fn GetMovementSpeed
  (return (Variables|Default|GetMySpeed)))

(fn GetMyFlashColor
  (return (Variables|Default|GetFlashColor)))