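; BP_IndicatorLight is an indicator lamp that briefly flashes in whatever color it is sent.
; The construction script creates a dynamic material instance on the lamp mesh.
; SendSignalColor tints and brightens that material, spawns a color-matched Niagara flash above the actor, then returns to dimmer gray after a short delay.
; The distance, item type, speed and flash color getters return only placeholder defaults.
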(event EventBeginPlay)

(event Collision|EventActorBeginOverlap
  (params (OtherActor :type Actor%20Object%20Reference)))

(event EventTick
  (params (DeltaSeconds :type Float%20%28single-precision%29)))

(event EventSendSignalColor
  (params (SignalColor :type Linear%20Color%20Structure))
  (bind (_r _g _b) (Utilities|Struct|BreakLinearColor SignalColor))
  (Rendering|Material|SetScalarParameterValue (Variables|Default|GetDynamicLampMat) "EmissiveStrength" 3e+01 :!class /Script/Engine.MaterialInstanceDynamic)
  (Rendering|Material|SetVectorParameterValue (Variables|Default|GetDynamicLampMat) "Base Color" SignalColor :!class /Script/Engine.MaterialInstanceDynamic)
  (bind _returnvalue (Niagara|SpawnSystematLocation "/Game/NS_LampFlash.NS_LampFlash" (+ (Transformation|GetActorLocation) "0, 0,90.000000")))
  (Niagara|SetNiagaraVariable(LinearColor) _returnvalue "FlashColor" (Utilities|Struct|MakeLinearColor _r _g _b 1.0))
  (Utilities|FlowControl|Delay 0.2)
  (Rendering|Material|SetScalarParameterValue (Variables|Default|GetDynamicLampMat) "EmissiveStrength" 1e+01 :!class /Script/Engine.MaterialInstanceDynamic)
  (Rendering|Material|SetVectorParameterValue (Variables|Default|GetDynamicLampMat) "Base Color" "(R=0.537500,G=0.537500,B=0.537500,A=1.000000)" :!class /Script/Engine.MaterialInstanceDynamic))

(fn ConstructionScript
  (bind _returnvalue (Rendering|Material|CreateDynamicMaterialInstance (Variables|Default|GetIndicatorLight) 0 "/Game/M_Indicator.M_Indicator" "None" :!class /Script/Engine.PrimitiveComponent))
  (Variables|Default|SetDynamicLampMat _returnvalue))

(fn GetCurrentDistance
  (return 0.0))

(fn GetItemType
  (return "None"))

(fn GetMovementSpeed
  (return 0.0))

(fn GetMyFlashColor
  (return ""))