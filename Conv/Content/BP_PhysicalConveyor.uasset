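; BP_PhysicalConveyor is a physics-driven conveyor that pushes tagged objects along its local forward axis.
; Every Tick, it finds actors tagged "Con" overlapping its box collision and applies a mass-independent force to their static mesh component.
; The force combines constant forward push with a sideways pull proportional to local Y offset, centring objects on the belt.
; It also raises linear damping to limit speed, without restoring it afterward.
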(event EventBeginPlay)

(event Collision|EventActorBeginOverlap
  (params (OtherActor :type Actor%20Object%20Reference)))

(event EventTick
  (params (DeltaSeconds :type Float%20%28single-precision%29))
  (for _array_element (Collision|GetOverlappingActors (Variables|Default|GetBox%20Collision) 0 :!class /Script/Engine.PrimitiveComponent)
    (Variables|Default|SetArray%20Element _array_element)
    (if (Actor|ActorHasTag (Variables|Default|GetArray%20Element) "Con")
      (Physics|AddForce (Actor|GetComponentbyClass (Variables|Default|GetArray%20Element) "/Script/Engine.StaticMeshComponent") (Math|Transform|TransformDirection (Transformation|GetActorTransform) (Math|Vector|MakeVector 8e+02 (* -10 (.Y (Math|Vector|BreakVector (Math|Transform|InverseTransformLocation (Transformation|GetActorTransform) (Transformation|GetActorLocation (Variables|Default|GetArray%20Element)))))) 0.0)) "None" true)
      (Class|PrimitiveComponent|SetLinearDamping (Actor|GetComponentbyClass (Variables|Default|GetArray%20Element) "/Script/Engine.StaticMeshComponent") 2.0))))

(fn ConstructionScript)